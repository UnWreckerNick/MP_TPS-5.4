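; BP_WeaponFX is an actor that plays Niagara muzzle flash, shell eject and tracer effects for weapon fire.
; WeaponFired spawns each system at its mesh socket only when missing or inactive, then flips a User.Trigger bool to reuse it.
; Impact positions set the flash direction and feed the tracer array.
; A retriggerable delay loop destroys the actor once all three auto-destroying systems are gone.
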(event Custom|WeaponFired
  (params (ImpactPositions :type Array%20of%20Vectors))
  (Variables|Default|SetImpactPositions ImpactPositions)
  (Utilities|FlowControl|Sequence
    (:then_0
      (Utilities|IsValid (Variables|Default|GetNS_MuzzleFlash)
        (:Is%20Valid
          (if (Components|Activation|IsActive (Variables|Default|GetNS_MuzzleFlash))
            _
            (else
              (bind _returnvalue (Niagara|SpawnSystemAttached (Variables|Default|GetMuzzleFleshFX) (Variables|Default|GetDefaultSceneRoot) "None" (.Location (Math|Transform|BreakTransform (Transformation|GetSocketTransform (Variables|Default|GetWeaponMesh) (Variables|Default|GetMuzzleSocket) "RTS_Component"))) "0.000000,90.000000,0.000000" "KeepRelativeOffset" true :!label _label))
              (Variables|Default|SetNS_MuzzleFlash _returnvalue)
              (Variables|Default|SetMuzzleFlash_Trigger false))))
        (:Is%20Not%20Valid
          (goto _label)))
      (Variables|Default|SetMuzzleFlash_Trigger (not (Variables|Default|GetMuzzleFlash_Trigger)))
      (Niagara|SetNiagaraVariable(Vector3) (Variables|Default|GetNS_MuzzleFlash) "User.Direction" (Math|Vector|Normalize (- (Utilities|Array|Get(acopy) (Variables|Default|GetImpactPositions)) (.Location (Math|Transform|BreakTransform (Transformation|GetSocketTransform (Variables|Default|GetWeaponMesh) (Variables|Default|GetMuzzleSocket) "RTS_Component"))))))
      (Class|NiagaraComponent|SetVariableBool (Variables|Default|GetNS_MuzzleFlash) "User.Trigger" (Variables|Default|GetMuzzleFlash_Trigger)))
    (:then_1
      (Utilities|IsValid (Variables|Default|GetNS_ShellEject)
        (:Is%20Valid
          (if (Components|Activation|IsActive (Variables|Default|GetNS_ShellEject))
            _
            (else
              (bind _returnvalue_2 (Niagara|SpawnSystemAttached "/Game/Effects/Particles/Weapons/NS_WeaponFire_ShellEject.NS_WeaponFire_ShellEject" (Variables|Default|GetDefaultSceneRoot) "None" (.Location (Math|Transform|BreakTransform (Transformation|GetSocketTransform (Variables|Default|GetWeaponMesh) (Variables|Default|GetShellEjectSocket) "RTS_Component"))) "0.000000,90.000000,0.000000" "KeepRelativeOffset" true :!label _label_2))
              (bind _output_get (Variables|Default|SetNS_ShellEject _returnvalue_2))
              (Class|NiagaraComponent|SetVariableStaticMesh _output_get "User.ShellEjectStaticMesh" (Variables|Default|GetShellEjectMesh))
              (Variables|Default|SetShellEject_Trigger false))))
        (:Is%20Not%20Valid
          (goto _label_2)))
      (Variables|Default|SetShellEject_Trigger (not (Variables|Default|GetShellEject_Trigger)))
      (Class|NiagaraComponent|SetVariableBool (Variables|Default|GetNS_ShellEject) "User.Trigger" (Variables|Default|GetShellEject_Trigger)))
    (:then_2
      (Utilities|IsValid (Variables|Default|GetNS_TracerFX)
        (:Is%20Valid
          (if (Components|Activation|IsActive (Variables|Default|GetNS_TracerFX))
            _
            (else
              (bind _returnvalue_3 (Niagara|SpawnSystemAttached (Variables|Default|GetTracerFX) (Variables|Default|GetDefaultSceneRoot) "None" (.Location (Math|Transform|BreakTransform (Transformation|GetSocketTransform (Variables|Default|GetWeaponMesh) (Variables|Default|GetMuzzleSocket) "RTS_Component"))) "0.000000,90.000000,0.000000" "KeepRelativeOffset" true :!label _label_3))
              (Variables|Default|SetNS_TracerFX _returnvalue_3)
              (Variables|Default|SetTracer_Trigger false))))
        (:Is%20Not%20Valid
          (goto _label_3)))
      (Variables|Default|SetTracer_Trigger (not (Variables|Default|GetTracer_Trigger)))
      (Class|NiagaraDataInterfaceArrayFunctionLibrary|SetNiagaraArrayVector (Variables|Default|GetNS_TracerFX) "User.ImpactPositions" (Variables|Default|GetImpactPositions))
      (Class|NiagaraComponent|SetVariableBool (Variables|Default|GetNS_TracerFX) "User.Trigger" (Variables|Default|GetTracer_Trigger)))
    (:then_3
      (Utilities|FlowControl|RetriggerableDelay 3.0 :!label _label_4)
      (if (Math|Boolean|ORBoolean (Utilities|IsValid (Variables|Default|GetNS_MuzzleFlash)) (Utilities|IsValid (Variables|Default|GetNS_ShellEject)) (Utilities|IsValid (Variables|Default|GetNS_TracerFX)))
        (goto _label_4)
        (else
          (Actor|DestroyActor))))))

(fn ConstructionScript)