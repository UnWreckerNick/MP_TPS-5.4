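; Game instance for a multiplayer third-person shooter, managing the player profile, menus, sessions and map travel.
; The profile persists through an SG_PlayerProfile save slot, loaded or created when the main menu opens.
; It creates or joins LAN-switchable sessions, hosts a listen-server lobby and server-travels with an accumulated URL options string.
; Pause toggling truly pauses only solo games, while multiplayer just shows or hides the pause menu.
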(event Custom|Start_SoloGame
  ;[1 1 1] Start solo
  (Variables|Default|SetisSoloGame true)
  (CallFunction|MakeOptionsScreen "NumConnectedPlayers" "1")
  (CallFunction|MakeOptionsScreen "IsSoloGame" (Utilities|String|ToString(Boolean) (Variables|Default|GetisSoloGame)))
  (CallFunction|MakeOptionsScreen "UseSeamlessTravel" (Utilities|String|ToString(Boolean) (Variables|Default|GetIsSeamlessTravelEnabled)))
  (CallFunction|MakeOptionsScreen "GameMode" "EndlessWave")
  (Game|OpenLevel(byObjectReference) "/Game/Maps/Map_01.Map_01" true "GameMode=EndlessWave"))

(event Custom|Change_PlayerName
  (params (PlayerName :type Text))
  ;[1 1 1] Change player name
  (Utilities|Struct|SetmembersinS_PlayerProfile (Variables|Default|GetPlayer%20Profile%20Info) PlayerName)
  (CallFunction|SaveProfile))

(event Custom|CreateMPSession
  ;[1 1 1] Multiplayer Sessions
  (Variables|Default|SetisSoloGame false)
  (|Session (Game|GetPlayerController 0) 4 (Variables|Default|GetisLanConnection) true
    (:OnSuccess
      (Game|OpenLevel(byObjectReference) "/Game/Maps/Menu/LobbyMenu_Map.LobbyMenu_Map" true "listen"))
    (:OnFailure
      (Development|PrintString "Failed to create session"))))

(event Custom|JoinMPSession
  (params (SessionResult :type Blueprint%20Session%20Result%20Structure))
  ;[1 1 1] Multiplayer Sessions
  (Variables|Default|SetisSoloGame false)
  (|JoinSession (Game|GetPlayerController 0) SessionResult
    (:OnFailure
      (Development|PrintString "Failed to join session"))))

(event Custom|TravelToMap
  (params (NumConnectedPlayers :type Integer) (MapName :type String))
  ;[1 1 1] Server Travel
  (CallFunction|MakeOptionsScreen "NumConnectedPlayers" (Utilities|String|ToString(Integer) NumConnectedPlayers))
  (CallFunction|MakeOptionsScreen "IsSoloGame" (Utilities|String|ToString(Boolean) (Variables|Default|GetisSoloGame)))
  (CallFunction|MakeOptionsScreen "UseSeamlessTravel" (Utilities|String|ToString(Boolean) (Variables|Default|GetIsSeamlessTravelEnabled)))
  (CallFunction|MakeOptionsScreen "GameMode" "EndlessWave")
  (Development|ExecuteConsoleCommand (Utilities|String|Append "servertravel " MapName (Variables|Default|GetOptionsString)) (Game|GetPlayerController 0)))

(event Custom|Reset_XP
  (Variables|Default|SetPlayer%20Profile%20Info (Utilities|Struct|MakeS_PlayerProfile (.playername (Variables|Default|GetPlayer%20Profile%20Info)) "Quinn_Blue" "/Game/Characters/Blueprints/BP_Player_Quinn_Blue.BP_Player_Quinn_Blue_C"))
  (CallFunction|SaveProfile))

(fn UIShowMainMenu
  (bind _returnvalue (Game|GetPlayerController 0))
  ;[1 1 1] Show Main Menu
  (CallFunction|CheckforSavedProfile)
  (Utilities|IsValid (Variables|Default|GetWB_MainMenu)
    (:Is%20Valid
      _)
    (:Is%20Not%20Valid
      (bind _returnvalue_2 (UserInterface|CreateWidget "/Game/Widgets/WB_MainMenu.WB_MainMenu_C" _returnvalue))
      (Variables|Default|SetWB_MainMenu _returnvalue_2)))
  (UserInterface|Viewport|AddtoViewport (Variables|Default|GetWB_MainMenu) 0)
  (Input|SetInputModeUIOnly _returnvalue 0 "DoNotLock" false)
  (Variables|/Script/Engine.PlayerController|SetbShowMouseCursor _returnvalue true)
  (return))

(fn CheckforSavedProfile
  ;[1 1 1] Check
  (bind _returnvalue (SaveGame|DoesSaveGameExist (Variables|Default|GetPlayerProfile_Slot)))
  (if _returnvalue
    (bind _sg_player_profile (CallFunction|LoadProfile))
    (Variables|Default|SetSG_PlayerProfile _sg_player_profile)
    (else
      (CallFunction|SaveProfile)))
  (return))

(fn LoadProfile
  ;[1 1 1] Load
  (bind _returnvalue (SaveGame|LoadGamefromSlot (Variables|Default|GetPlayerProfile_Slot)))
  (bind _assg_player_profile (Utilities|Casting|CastToSG_PlayerProfile _returnvalue))
  (Variables|Default|SetPlayer%20Profile%20Info (Variables|/Game/SavedData/SG_PlayerProfile.SG_PlayerProfile_C|GetPlayerProfile _assg_player_profile))
  (return _assg_player_profile))

(fn SaveProfile
  ;[1 1 1] Save
  (Utilities|IsValid (Variables|Default|GetSG_PlayerProfile)
    (:Is%20Valid
      _)
    (:Is%20Not%20Valid
      (bind _returnvalue (SaveGame|CreateSaveGameObject "/Game/SavedData/SG_PlayerProfile.SG_PlayerProfile_C"))
      (Variables|Default|SetSG_PlayerProfile _returnvalue)))
  (Variables|/Game/SavedData/SG_PlayerProfile.SG_PlayerProfile_C|SetPlayerProfile (Variables|Default|GetSG_PlayerProfile) (Variables|Default|GetPlayer%20Profile%20Info))
  (SaveGame|SaveGametoSlot (Variables|Default|GetSG_PlayerProfile) (Variables|Default|GetPlayerProfile_Slot))
  (return))

(fn UIShowMPMenu
  ;[1 1 1] Show Main Menu
  (Utilities|IsValid (Variables|Default|GetWB_MPMenu)
    (:Is%20Valid
      _)
    (:Is%20Not%20Valid
      (bind _returnvalue (UserInterface|CreateWidget "/Game/Widgets/WB_MPMenu.WB_MPMenu_C" (Game|GetPlayerController 0)))
      (Variables|Default|SetWB_MPMenu _returnvalue)))
  (UserInterface|Viewport|AddtoViewport (Variables|Default|GetWB_MPMenu) 0)
  (return))

(fn ChangeConnectionType
  (if (Variables|Default|GetisLanConnection)
    (Variables|Default|SetisLanConnection false)
    (else
      (Variables|Default|SetisLanConnection true)))
  (return (Variables|Default|GetisLanConnection)))

(fn UIShowPauseMenu
  (bind _returnvalue (Game|GetPlayerController 0))
  (Utilities|IsValid 0
    (:Is%20Valid
      _)
    (:Is%20Not%20Valid
      (bind _returnvalue_2 (UserInterface|CreateWidget "/Game/Widgets/WB_PauseMenu.WB_PauseMenu_C" _returnvalue))
      (Variables|Default|SetWB_PauseMenu _returnvalue_2)))
  (UserInterface|Viewport|AddtoViewport (Variables|Default|GetWB_PauseMenu) 0)
  (Input|SetInputModeUIOnly _returnvalue 0 "DoNotLock" false)
  (Variables|/Script/Engine.PlayerController|SetbShowMouseCursor _returnvalue true)
  (return))

(fn TogglePauseGame
  (bind _returnvalue (Game|GetPlayerController 0))
  (if (Variables|Default|GetisSoloGame)
    (if (Game|IsGamePaused)
      (bind _returnvalue_2 (Game|SetGamePaused false))
      (LocalVariables|SetLocal_IsGamePaused _returnvalue_2)
      (Widget|RemovefromParent (Variables|Default|GetWB_PauseMenu) :!label _label)
      (Input|SetInputModeGameOnly _returnvalue false)
      (Variables|/Script/Engine.PlayerController|SetbShowMouseCursor _returnvalue false)
      (bind _asbp_mptps_player_controller (Utilities|Casting|CastToBP_MPTPS_PlayerController _returnvalue))
      (Default|UnHideIngameHUD _asbp_mptps_player_controller)
      (else
        (bind _returnvalue_3 (Game|SetGamePaused true))
        (LocalVariables|SetLocal_IsGamePaused _returnvalue_3)
        (CallFunction|UIShowPauseMenu :!label _label_2)))
    (elif (Variables|Default|GetMP_IsPauseMenuVisible)
      (Variables|Default|SetMP_IsPauseMenuVisible false)
      (goto _label)
      (else
        (Variables|Default|SetMP_IsPauseMenuVisible true)
        (LocalVariables|SetLocal_IsGamePaused true)
        (goto _label_2))))
  (return (LocalVariables|GetLocal_IsGamePaused)))

(fn MakeOptionsScreen
  (params (NewOption :type String) (NewSetting :type String))
  (Variables|Default|SetOptionsString (Utilities|String|Append (Variables|Default|GetOptionsString) "?" NewOption "=" NewSetting))
  (return))