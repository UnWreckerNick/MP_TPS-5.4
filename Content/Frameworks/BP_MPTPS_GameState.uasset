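; Game state for a multiplayer third-person shooter that replicates the player name list and match countdown to each player's in-game HUD.
; On BeginPlay it caches the local player controller.
; Update events set the replicated variables, and their RepNotify functions push the new values into that controller's HUD widget when the controller is valid.
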(event Custom|Update_HUD_PlayerNames
  (params (All_PlayerNames :type Array%20of%20Texts))
  (Variables|Default|SetAll_PlayerNames All_PlayerNames))

(event Custom|Update_HUDMatchTimer
  (params (MatchTimeLeftSeconds :type Integer))
  (Variables|Default|SetMatchTimeLeftSeconds MatchTimeLeftSeconds))

(event EventBeginPlay
  (bind _asbp_mptps_player_controller (Utilities|Casting|CastToBP_MPTPS_PlayerController (Game|GetPlayerController 0)))
  (Variables|Default|SetBP_MPTPS_PlayerController _asbp_mptps_player_controller))

(fn ConstructionScript)

(fn OnRepAllPlayerNames
  (bind _bp_mptps_playercontroller (Variables|Default|GetBP_MPTPS_PlayerController)
    (:then
      (Default|UpdatePlayerNames (Variables|/Game/Frameworks/BP_MPTPS_PlayerController.BP_MPTPS_PlayerController_C|GetWB_IngameHUD _bp_mptps_playercontroller) (Variables|Default|GetAll_PlayerNames)))
    (:else)))

(fn OnRepMatchTimeLeftSeconds
  (bind _bp_mptps_playercontroller (Variables|Default|GetBP_MPTPS_PlayerController)
    (:then
      (Default|UpdateMatchTimer (Variables|/Game/Frameworks/BP_MPTPS_PlayerController.BP_MPTPS_PlayerController_C|GetWB_IngameHUD _bp_mptps_playercontroller) (Variables|Default|GetMatchTimeLeftSeconds)))
    (:else)))