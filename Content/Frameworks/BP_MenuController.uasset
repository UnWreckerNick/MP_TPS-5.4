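; Player controller for the multiplayer lobby menus, handling lobby, character, loadout and loading-screen widgets, chat and ready state.
; It loads the player profile from a save slot, saves character, skin and weapon picks, and sends lobby updates through server events to BP_MenuGameMode.
; Update events refresh the lobby widget.
; Menu switches blend the camera between lobby character view targets, and the loadout view previews weapons while hiding other players' characters.
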(event Custom|EndClientSession
  (|DestroySession self
    (:then
      (Game|OpenLevel(byObjectReference) "/Game/Maps/Menu/MainMenu_Map.MainMenu_Map"))))

(event Custom|CreateLobbyMenu
  (CallFunction|UIShowLobbyMenu))

(event Custom|Server_PreviewLockedCharacter
  (params (CharacterRowName :type Name) (ModelName :type Name) (SkinName :type Name))
  (bind _asbp_menu_game_mode (Utilities|Casting|CastToBP_MenuGameMode (Game|GetGameMode)))
  (Default|PreviewCharacterforController _asbp_menu_game_mode self CharacterRowName ModelName SkinName))

(event Custom|Server_SetViewTargetCharacter
  ;[1 1 1] View Target
  (Game|Player|SetViewTargetwithBlend (Variables|/Script/Engine.ChildActorComponent|GetChildActor (Variables|/Game/Gameplay/Lobby/BP_LobbyCharacter.BP_LobbyCharacter_C|GetViewTarget (Variables|Default|GetBP_LobbyCharacter))) 0.5 "VTBlend_Linear" 0.0 false))

(event Custom|LeaveLoadoutMenu
  (bind _bp_lobbycharacter (Variables|Default|GetBP_LobbyCharacter))
  (bind _player_profile (Variables|Default|GetPlayer%20Profile))
  ;[1 1 1] Loadout menu
  (Components|SkeletalMesh|SetSkeletalMeshAsset (Variables|/Game/Gameplay/Lobby/BP_LobbyCharacter.BP_LobbyCharacter_C|GetWeaponMesh _bp_lobbycharacter) 0)
  (bind _returnvalue (Utilities|GetDataTableRow "/Game/Characters/Blueprints/DT_CharacterCustomisation.DT_CharacterCustomisation" (.characterrowname _player_profile))
    (:then
      (Components|Animation|PlayAnimation (Variables|/Game/Gameplay/Lobby/BP_LobbyCharacter.BP_LobbyCharacter_C|GetCharacterMesh _bp_lobbycharacter) (.LobbyAnim (Utilities|Struct|BreakS_ModelsAndSkins (.Value (Utilities|Map|Find (.ModelsAndSkins (Utilities|Struct|BreakS_CharacterCustomisation _returnvalue)) (.modelname _player_profile))))) true)
      (bind _outactors (Actor|GetAllActorsOfClass "/Game/Gameplay/Lobby/BP_LobbyCharacter.BP_LobbyCharacter_C"))
      (for _array_element _outactors
        (if (!= _array_element (Variables|Default|GetBP_LobbyCharacter))
          (Rendering|SetVisibility (Variables|/Game/Gameplay/Lobby/BP_LobbyCharacter.BP_LobbyCharacter_C|GetCharacterMesh _array_element) true false)
          (Rendering|SetVisibility (Variables|/Game/Gameplay/Lobby/BP_LobbyCharacter.BP_LobbyCharacter_C|GetPlayerName _array_element) true false))))))

(event Custom|EnterLoadoutMenu
  (bind _bp_lobbycharacter (Variables|Default|GetBP_LobbyCharacter))
  ;[1 1 1] Loadout menu
  (bind _returnvalue (Utilities|GetDataTableRow "/Game/Weapons/DT_WeaponInfo.DT_WeaponInfo" (Utilities|Array|Get(acopy) (.weapon_loadout (Variables|Default|GetPlayer%20Profile))))
    (:then
      (Components|SkeletalMesh|SetSkeletalMeshAsset (Variables|/Game/Gameplay/Lobby/BP_LobbyCharacter.BP_LobbyCharacter_C|GetWeaponMesh _bp_lobbycharacter) (.WeaponMesh (Utilities|Struct|BreakS_WeaponInfo _returnvalue)))
      (Components|Animation|PlayAnimation (Variables|/Game/Gameplay/Lobby/BP_LobbyCharacter.BP_LobbyCharacter_C|GetCharacterMesh _bp_lobbycharacter) (.Character_Hip_Idle (Utilities|Struct|BreakS_WeaponInfo _returnvalue)) false)
      (bind _outactors (Actor|GetAllActorsOfClass "/Game/Gameplay/Lobby/BP_LobbyCharacter.BP_LobbyCharacter_C"))
      (for _array_element _outactors
        (if (!= _array_element (Variables|Default|GetBP_LobbyCharacter))
          (Rendering|SetVisibility (Variables|/Game/Gameplay/Lobby/BP_LobbyCharacter.BP_LobbyCharacter_C|GetCharacterMesh _array_element) false false)
          (Rendering|SetVisibility (Variables|/Game/Gameplay/Lobby/BP_LobbyCharacter.BP_LobbyCharacter_C|GetPlayerName _array_element) false false))))))

(event Custom|Update_LoadoutCharacter
  (params (WeaponRowName :type Name))
  (bind _bp_lobbycharacter (Variables|Default|GetBP_LobbyCharacter))
  (bind _bp_lobbycharacter_2 (Variables|Default|GetBP_LobbyCharacter))
  ;[1 1 1] UPDATE
  ;;[1 1 1] Loadout
  (if (== WeaponRowName "")
    (Components|SkeletalMesh|SetSkeletalMeshAsset (Variables|/Game/Gameplay/Lobby/BP_LobbyCharacter.BP_LobbyCharacter_C|GetWeaponMesh _bp_lobbycharacter_2) 0)
    (Components|Animation|PlayAnimation (Variables|/Game/Gameplay/Lobby/BP_LobbyCharacter.BP_LobbyCharacter_C|GetCharacterMesh _bp_lobbycharacter_2) "/Game/Characters/Heroes/Mannequin/Animations/Locomotion/Unarmed/MF_Unarmed_Idle_Ready.MF_Unarmed_Idle_Ready" true)
    (else
      (bind _returnvalue (Utilities|GetDataTableRow "/Game/Weapons/DT_WeaponInfo.DT_WeaponInfo" WeaponRowName)
        (:then
          (Components|SkeletalMesh|SetSkeletalMeshAsset (Variables|/Game/Gameplay/Lobby/BP_LobbyCharacter.BP_LobbyCharacter_C|GetWeaponMesh _bp_lobbycharacter) (.WeaponMesh (Utilities|Struct|BreakS_WeaponInfo _returnvalue)))
          (Components|Animation|PlayAnimation (Variables|/Game/Gameplay/Lobby/BP_LobbyCharacter.BP_LobbyCharacter_C|GetCharacterMesh _bp_lobbycharacter) (.Character_Hip_Idle (Utilities|Struct|BreakS_WeaponInfo _returnvalue)) true))))))

(event Custom|Server_UpdatePlayerReady
  (params (IsReady :type Boolean))
  ;[1 1 1] UPDATE
  ;;[1 1 1] Player Ready
  (bind _asbp_menu_game_mode (Utilities|Casting|CastToBP_MenuGameMode (Game|GetGameMode)))
  (Default|SetPlayerReady _asbp_menu_game_mode self IsReady))

(event Custom|UpdatePlayerReady
  (params (PlayerReady :type Array%20of%20Booleans))
  (bind _wb_lobbymenu (Variables|Default|GetWB_LobbyMenu))
  ;[1 1 1] UPDATE
  ;;[1 1 1] Player Ready
  (Utilities|IsValid _wb_lobbymenu
    (:Is%20Valid
      (Default|UpdatePlayersReady _wb_lobbymenu PlayerReady))))

(event Custom|UpdateGameMode
  (params (GameMode :type E_GameModes%20Enum :default "NewEnumerator0"))
  (bind _wb_lobbymenu (Variables|Default|GetWB_LobbyMenu))
  ;[1 1 1] UPDATE
  ;;[1 1 1] Game Mode
  (Utilities|IsValid _wb_lobbymenu
    (:Is%20Valid
      (Default|UpdateGameMode _wb_lobbymenu (Utilities|String|EnumtoString GameMode)))))

(event Custom|Update_ChatBox
  (params (Message :type Text))
  (bind _wb_lobbymenu (Variables|Default|GetWB_LobbyMenu))
  (Utilities|IsValid _wb_lobbymenu
    (:Is%20Valid
      (Default|AddChatMessage _wb_lobbymenu Message))))

(event Custom|Server_SendCharMessage
  (params (Message :type Text))
  (bind _asbp_menu_game_mode (Utilities|Casting|CastToBP_MenuGameMode (Game|GetGameMode)))
  (Default|SendChatMessage _asbp_menu_game_mode Message))

(event Custom|InitialSetup
  (if (Variables|Default|GetIsSlotLoaded) :!label _label
    (CallFunction|LoadSaveProfile)
    (Variables|Default|SetIsProfileLoaded true)
    (CallFunction|ServerUpdateLobby (Variables|Default|GetPlayer%20Profile))
    (else
      (Utilities|FlowControl|Delay 0.05)
      (goto _label))))

(event Custom|UpdatePlayerNames
  (params (PlayerProfiles :type Array%20of%20S%20Player%20Profile%20Structures))
  (bind _wb_lobbymenu (Variables|Default|GetWB_LobbyMenu))
  ;[1 1 1] UPDATE
  ;;[1 1 1] PlayerNames
  (Utilities|IsValid _wb_lobbymenu
    (:Is%20Valid
      (Default|ClearPlayerNames _wb_lobbymenu)
      (Default|UpdatePlayerNames _wb_lobbymenu PlayerProfiles))))

(event Custom|Server_UpdateLobby
  (params (PlayerProfile :type S%20Player%20Profile%20Structure))
  ;[1 1 1] UPDATE
  ;;[1 1 1] Lobby
  (Variables|Default|SetPlayer%20Profile PlayerProfile)
  (bind _asbp_menu_game_mode (Utilities|Casting|CastToBP_MenuGameMode (Game|GetGameMode)))
  (Default|UpdateLobby _asbp_menu_game_mode true true true true true))

(event Custom|CreateLoadingScreen
  (CallFunction|UIShowLoadingScreen))

(event Custom|UpdateLevelSelection
  (params (LevelRowName :type Name))
  (bind _wb_lobbymenu (Variables|Default|GetWB_LobbyMenu))
  ;[1 1 1] UPDATE
  ;;[1 1 1] Level
  (Utilities|IsValid _wb_lobbymenu
    (:Is%20Valid
      (Default|UpdateLevelSelection _wb_lobbymenu LevelRowName))))

(event Custom|Server_SetViewTarget_Normal
  ;[1 1 1] View Target
  (Game|Player|SetViewTargetwithBlend (Pawn|GetControlledPawn) 0.5 "VTBlend_Linear" 0.0 false))

(event Custom|Server_SetViewTargetWeapon
  ;[1 1 1] View Target
  (Game|Player|SetViewTargetwithBlend (Variables|/Script/Engine.ChildActorComponent|GetChildActor (Variables|/Game/Gameplay/Lobby/BP_LobbyCharacter.BP_LobbyCharacter_C|GetViewTargetWeapon (Variables|Default|GetBP_LobbyCharacter))) 0.5 "VTBlend_Linear" 0.0 false))

(event Custom|Server_UpdateSelectedCharacter
  (params (Player%20Profile :type S%20Player%20Profile%20Structure))
  ;[1 1 1] UPDATE
  ;;[1 1 1] Selected Characther
  (bind _output_get (Variables|Default|SetPlayer%20Profile Player%20Profile))
  (bind _asbp_menu_game_mode (Utilities|Casting|CastToBP_MenuGameMode (Game|GetGameMode)))
  (Default|UpdateCharacterforController _asbp_menu_game_mode self _output_get))

(event EventBeginPlay
  ;[0.4719 1 0.3926] Begin Play
  (if (Pawn|IsLocalController)
    (Variables|Default|SetbShowMouseCursor true)
    (Input|SetInputModeUIOnly self 0 "DoNotLock" false)
    (bind _asbp_mptps_game_instance (Utilities|Casting|CastToBP_MPTPS_GameInstance (Game|GetGameInstance)))
    (Variables|Default|SetPlayerProfileSlot (Variables|/Game/Frameworks/BP_MPTPS_GameInstance.BP_MPTPS_GameInstance_C|GetPlayerProfile_Slot _asbp_mptps_game_instance))
    (Variables|Default|SetIsSlotLoaded true)))

(fn ConstructionScript)

(fn UIShowLobbyMenu
  (Utilities|IsValid (Variables|Default|GetWB_LobbyMenu)
    (:Is%20Valid
      _)
    (:Is%20Not%20Valid
      (bind _returnvalue (UserInterface|CreateWidget "/Game/Widgets/WB_LobbyMenu.WB_LobbyMenu_C" self))
      (Variables|Default|SetWB_LobbyMenu _returnvalue)))
  (UserInterface|Viewport|AddtoViewport (Variables|Default|GetWB_LobbyMenu) 0)
  (if (Variables|Default|GetIsInLoadoutMenu)
    (CallFunction|LeaveLoadoutMenu)
    (Variables|Default|SetIsInLoadoutMenu false))
  (Networking|SwitchHasAuthority
    (:Authority
      (Game|Player|SetViewTargetwithBlend (Pawn|GetControlledPawn) 0.5 "VTBlend_Linear" 0.0 false))
    (:Remote
      (CallFunction|ServerSetViewTargetNormal)))
  (return))

(fn LoadSaveProfile
  (LocalVariables|SetLocal_SlotName (Variables|Default|GetPlayerProfileSlot))
  (bind _returnvalue (SaveGame|DoesSaveGameExist (LocalVariables|GetLocal_SlotName)))
  (if _returnvalue
    _
    (else
      (bind _returnvalue_2 (SaveGame|CreateSaveGameObject "/Game/SavedData/SG_PlayerProfile.SG_PlayerProfile_C"))
      (SaveGame|SaveGametoSlot _returnvalue_2 (LocalVariables|GetLocal_SlotName))))
  (bind _returnvalue_3 (SaveGame|LoadGamefromSlot (LocalVariables|GetLocal_SlotName)))
  (bind _assg_player_profile (Utilities|Casting|CastToSG_PlayerProfile _returnvalue_3))
  (Variables|Default|SetPlayer%20Profile (Variables|/Game/SavedData/SG_PlayerProfile.SG_PlayerProfile_C|GetPlayerProfile _assg_player_profile))
  (return))

(fn UIShowLoadingScreen
  (Viewport|RemoveAllWidgets)
  (Utilities|IsValid (Variables|Default|GetWB_LoadingScreen)
    (:Is%20Valid
      _)
    (:Is%20Not%20Valid
      (bind _returnvalue (UserInterface|CreateWidget "/Game/Widgets/WB_LoadingScreen.WB_LoadingScreen_C" self))
      (Variables|Default|SetWB_LoadingScreen _returnvalue)))
  (UserInterface|Viewport|AddtoViewport (Variables|Default|GetWB_LoadingScreen) 0)
  (return))

(fn UIShowCharacterMenu
  (Utilities|IsValid (Variables|Default|GetWB_CharacterMenu)
    (:Is%20Valid
      _)
    (:Is%20Not%20Valid
      (bind _returnvalue (UserInterface|CreateWidget "/Game/Widgets/WB_CharacterMenu.WB_CharacterMenu_C" self))
      (Variables|Default|SetWB_CharacterMenu _returnvalue)))
  (UserInterface|Viewport|AddtoViewport (Variables|Default|GetWB_CharacterMenu) 0)
  (Networking|SwitchHasAuthority
    (:Authority
      (Game|Player|SetViewTargetwithBlend (Variables|/Script/Engine.ChildActorComponent|GetChildActor (Variables|/Game/Gameplay/Lobby/BP_LobbyCharacter.BP_LobbyCharacter_C|GetViewTarget (Variables|Default|GetBP_LobbyCharacter))) 0.5 "VTBlend_Linear" 0.0 false))
    (:Remote
      (CallFunction|ServerSetViewTargetCharacter)))
  (return))

(fn SaveSelectedCharacter
  (params (CharacterRowName :type Name) (Player%20Profile%20Character%20Class :type Actor%20Class%20Reference))
  (Utilities|Struct|SetmembersinS_PlayerProfile (Variables|Default|GetPlayer%20Profile) CharacterRowName Player%20Profile%20Character%20Class "Default" "Default")
  (Utilities|IsValid (Variables|Default|GetSG_PlayerProfile)
    (:Is%20Valid
      _)
    (:Is%20Not%20Valid
      (bind _returnvalue (SaveGame|CreateSaveGameObject "/Game/SavedData/SG_PlayerProfile.SG_PlayerProfile_C"))
      (Variables|Default|SetSG_PlayerProfile _returnvalue)
      (Variables|/Game/SavedData/SG_PlayerProfile.SG_PlayerProfile_C|SetPlayerProfile (Variables|Default|GetSG_PlayerProfile) (Variables|Default|GetPlayer%20Profile))))
  (SaveGame|SaveGametoSlot (Variables|Default|GetSG_PlayerProfile) (Variables|Default|GetPlayerProfileSlot))
  (CallFunction|ServerUpdateSelectedCharacter (Variables|Default|GetPlayer%20Profile))
  (return))

(fn SaveSelectedModel
  (params (ModelName :type Name))
  (Utilities|Struct|SetmembersinS_PlayerProfile (Variables|Default|GetPlayer%20Profile) ModelName)
  (Utilities|IsValid (Variables|Default|GetSG_PlayerProfile)
    (:Is%20Valid
      _)
    (:Is%20Not%20Valid
      (bind _returnvalue (SaveGame|CreateSaveGameObject "/Game/SavedData/SG_PlayerProfile.SG_PlayerProfile_C"))
      (Variables|Default|SetSG_PlayerProfile _returnvalue)
      (Variables|/Game/SavedData/SG_PlayerProfile.SG_PlayerProfile_C|SetPlayerProfile (Variables|Default|GetSG_PlayerProfile) (Variables|Default|GetPlayer%20Profile))))
  (SaveGame|SaveGametoSlot (Variables|Default|GetSG_PlayerProfile) (Variables|Default|GetPlayerProfileSlot))
  (CallFunction|ServerUpdateSelectedCharacter (Variables|Default|GetPlayer%20Profile))
  (return))

(fn SaveSelectedSkin
  (params (SkinName :type Name))
  (Utilities|Struct|SetmembersinS_PlayerProfile (Variables|Default|GetPlayer%20Profile) SkinName)
  (Utilities|IsValid (Variables|Default|GetSG_PlayerProfile)
    (:Is%20Valid
      _)
    (:Is%20Not%20Valid
      (bind _returnvalue (SaveGame|CreateSaveGameObject "/Game/SavedData/SG_PlayerProfile.SG_PlayerProfile_C"))
      (Variables|Default|SetSG_PlayerProfile _returnvalue)
      (Variables|/Game/SavedData/SG_PlayerProfile.SG_PlayerProfile_C|SetPlayerProfile (Variables|Default|GetSG_PlayerProfile) (Variables|Default|GetPlayer%20Profile))))
  (SaveGame|SaveGametoSlot (Variables|Default|GetSG_PlayerProfile) (Variables|Default|GetPlayerProfileSlot))
  (CallFunction|ServerUpdateSelectedCharacter (Variables|Default|GetPlayer%20Profile))
  (return))

(fn UIShowLoadoutMenu
  (Utilities|IsValid (Variables|Default|GetWB_LoadoutMenu)
    (:Is%20Valid
      _)
    (:Is%20Not%20Valid
      (bind _returnvalue (UserInterface|CreateWidget "/Game/Widgets/WB_LoadoutMenu.WB_LoadoutMenu_C" self))
      (Variables|Default|SetWB_LoadoutMenu _returnvalue)))
  (UserInterface|Viewport|AddtoViewport (Variables|Default|GetWB_LoadoutMenu) 0)
  (Variables|Default|SetIsInLoadoutMenu true)
  (Networking|SwitchHasAuthority
    (:Authority
      (Game|Player|SetViewTargetwithBlend (Variables|/Script/Engine.ChildActorComponent|GetChildActor (Variables|/Game/Gameplay/Lobby/BP_LobbyCharacter.BP_LobbyCharacter_C|GetViewTargetWeapon (Variables|Default|GetBP_LobbyCharacter))) 0.5 "VTBlend_Linear" 0.0 false))
    (:Remote
      (CallFunction|ServerSetViewTargetWeapon)))
  (CallFunction|EnterLoadoutMenu)
  (return))

(fn SaveSelectedLoadout
  (params (WeaponRowName :type Name) (InventoryIndex :type Integer))
  (bind _output_get (LocalVariables|SetLocal_PlayerLoadout (.weapon_loadout (Variables|Default|GetPlayer%20Profile))))
  (Utilities|Array|SetArrayElem _output_get InventoryIndex WeaponRowName)
  (Utilities|Struct|SetmembersinS_PlayerProfile (Variables|Default|GetPlayer%20Profile) (LocalVariables|GetLocal_PlayerLoadout))
  (Utilities|IsValid (Variables|Default|GetSG_PlayerProfile)
    (:Is%20Valid
      _)
    (:Is%20Not%20Valid
      (bind _returnvalue (SaveGame|CreateSaveGameObject "/Game/SavedData/SG_PlayerProfile.SG_PlayerProfile_C"))
      (Variables|Default|SetSG_PlayerProfile _returnvalue)
      (Variables|/Game/SavedData/SG_PlayerProfile.SG_PlayerProfile_C|SetPlayerProfile (Variables|Default|GetSG_PlayerProfile) (Variables|Default|GetPlayer%20Profile))))
  (SaveGame|SaveGametoSlot (Variables|Default|GetSG_PlayerProfile) (Variables|Default|GetPlayerProfileSlot))
  (return))