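; BP_MPTPS_PlayerState is a player state that holds a player's profile and name.
; On BeginPlay, the server caches the owning BP_MPTPS_PlayerController and polls it every tick until its profile is loaded.
; It then copies the profile struct into its own variables and sets MyPlayerName from it.
; The CopyProperties event is empty.
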(event EventBeginPlay
  (if (Networking|IsServer)
    (bind _asbp_mptps_player_controller (Utilities|Casting|CastToBP_MPTPS_PlayerController (Game|GetPlayerController)))
    (bind _output_get (Variables|Default|SetBP_MPTPSPlayerController _asbp_mptps_player_controller))
    (if (Variables|/Game/Frameworks/BP_MPTPS_PlayerController.BP_MPTPS_PlayerController_C|GetIsProfileLoaded _output_get) :!label _label
      (bind _output_get_2 (Variables|Default|SetS_PlayerProfile (Variables|/Game/Frameworks/BP_MPTPS_PlayerController.BP_MPTPS_PlayerController_C|GetS_PlayerProfile _output_get)))
      (Variables|Default|SetMyPlayerName (.PlayerName (Utilities|Struct|BreakS_PlayerProfile _output_get_2)))
      (else
        (Utilities|FlowControl|DelayUntilNextTick)
        (goto _label)))))

(event EventCopyProperties
  (params (NewPlayerState :type Player%20State%20Object%20Reference)))

(fn ConstructionScript)