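; Game mode for a multiplayer third-person shooter that runs solo or multiplayer Endless Wave and timed Free for All matches.
; URL options set the rules; it waits for all expected players, then spawns their profile characters at tagged PlayerStarts.
; Endless Wave spawns escalating AI waves until all players die.
; Free for All respawns players at cooldown-guarded points, ending on timer or when a victim's deaths reach ScoreLimit.
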(event Custom|LevelStart_EndlessWave
  ;[1 1 1] Level Start Endless Wave
  (CallFunction|UpdateGameStateNames)
  (for _array_element (Variables|Default|GetAll_ConnectedControllers)
    (Default|GameStartCountdown _array_element))
  (Utilities|FlowControl|Delay 3.0)
  (for _array_element_2 (Variables|Default|GetAll_ConnectedControllers)
    (Default|EnableAllInput _array_element_2))
  (bind _outactors (Actor|GetAllActorsOfClasswithTag "/Game/Gameplay/BP_SpawnPoint_AI.BP_SpawnPoint_AI_C" "EndlessWave"))
  (Variables|Default|SetAll_SpawnPoints _outactors)
  (Variables|Default|SetGM_EW_WaveNumber 0)
  (Variables|Default|SetGM_EW_EnemiesHealthThisWave 1e+02)
  (CallFunction|StartWave))

(event Custom|GM_PVP_GameOver
  (params (IsScoreLimit :type Boolean) (IsTimeLimit :type Boolean) (Winner :type BP%20MPTPS%20Player%20Controller%20Object%20Reference))
  ;[1 1 1] PVP GameOver
  (for _array_element (Variables|Default|GetAll_ConnectedControllers)
    (Variables|/Game/Frameworks/BP_MPTPS_PlayerController.BP_MPTPS_PlayerController_C|SetIsGameOver _array_element true)
    (Default|ControllerDisableInput _array_element)
    (Default|UIShowGameOverScreen _array_element 0 true (== _array_element Winner) IsScoreLimit IsTimeLimit))
  (Utilities|FlowControl|Delay 3.0)
  (for _array_element_2 (Variables|Default|GetAll_ConnectedControllers)
    (Default|ClientToggleScoreboard _array_element_2 true))
  (Utilities|FlowControl|Delay 1e+01)
  (Development|ExecuteConsoleCommand "servertravel LobbyMenu_Map" (Game|GetPlayerController 0)))

(event Custom|StartWave
  ;[1 1 1] Start wave
  (Math|Integer|IncrementInt (Variables|Default|GetGM_EW_WaveNumber)
    (:%20%20
      (for _array_element (Variables|Default|GetAll_ConnectedControllers)
        (Default|ClientHUDStartNewWave _array_element (Variables|Default|GetGM_EW_WaveNumber)))
      (bind _spawncount (CallFunction|GMEWGetEnemyCount (Variables|Default|GetGM_EW_WaveNumber) (Utilities|Array|Length (Variables|Default|GetAll_ConnectedControllers))))
      (Variables|Default|SetGM_EW_EnemiesNumberThisWave _spawncount)
      (bind _enemyhealth (CallFunction|GMEWGetEnemyHealth (Variables|Default|GetGM_EW_WaveNumber)))
      (Variables|Default|SetGM_EW_EnemiesHealthThisWave _enemyhealth)
      (CallFunction|WaveSpawner))))

(event Custom|WaveSpawner
  ;[1 1 1] Wave spawn
  (Variables|Default|SetGM_EW_SpawnCount 0)
  (bind _returnvalue (Game|SpawnActorfromClass "/Game/AI/BP_AI_Minion_Base.BP_AI_Minion_Base_C" (Transformation|GetActorTransform (.OutItem (Utilities|Array|Random (Variables|Default|GetAll_SpawnPoints)))) "Undefined" "MultiplyWithRoot" 0 0 :!label _label))
  (Utilities|IsValid _returnvalue
    (:Is%20Valid
      (Math|Integer|IncrementInt (Variables|Default|GetGM_EW_SpawnCount)
        (:%20%20
          (CallFunction|GMEWSetupEnemy _returnvalue)
          (if (== (Variables|Default|GetGM_EW_SpawnCount) (Variables|Default|GetGM_EW_EnemiesNumberThisWave))
            (Variables|Default|SetGM_EW_WaitForWaveEnd false :!label _label_2)
            (bind _outactors (Actor|GetAllActorsOfClass "/Game/AI/BP_AI_Minion_Base.BP_AI_Minion_Base_C"))
            (bind _array_element (Utilities|Array|ForEachLoopwithBreak _outactors :!label _label_3)
              (:LoopBody
                (if (Variables|/Game/AI/BP_AI_Minion_Base.BP_AI_Minion_Base_C|GetIsAlive _array_element)
                  (Variables|Default|SetGM_EW_WaitForWaveEnd true)
                  (goto _label_3 Break)))
              (:Completed
                (if (Variables|Default|GetGM_EW_WaitForWaveEnd)
                  (Utilities|FlowControl|Delay 1.0)
                  (goto _label_2)
                  (else
                    (CallFunction|WaveIntermission)))))
            (else
              (Utilities|FlowControl|Delay (Math|Conversions|ToFloat(Integer) (/ (Math|Random|RandomIntegerinRange 15 25) 10)))
              (goto _label))))))
    (:Is%20Not%20Valid
      (Utilities|FlowControl|Delay 0.2)
      (goto _label))))

(event Custom|WaveIntermission
  ;[1 1 1] Wave spawn
  (Development|PrintString "Wave ended: Intermission" true true "(R=0.000000,G=0.660000,B=1.000000,A=1.000000)" 5.0)
  (Utilities|FlowControl|Delay 3.0)
  (Development|PrintString "Intermission ended: New wave started" true true "(R=0.000000,G=0.660000,B=1.000000,A=1.000000)" 5.0)
  (CallFunction|StartWave))

(event Custom|GM_EW_GameOver
  ;[1 1 1] EndlessWave GameOver
  (for _array_element (Variables|Default|GetAll_ConnectedControllers)
    (Default|UIShowGameOverScreen _array_element (- (Variables|Default|GetGM_EW_WaveNumber) 1) false false false false))
  (Utilities|FlowControl|Delay 5.0)
  (if (Variables|Default|GetIsSoloGame)
    (Development|ExecuteConsoleCommand "servertravel MainMenu_Map" (Game|GetPlayerController 0))
    (else
      (Development|ExecuteConsoleCommand "servertravel LobbyMenu_Map" (Game|GetPlayerController 0)))))

(event Custom|LevelStart_FreeForAll
  (bind _matchduration (Variables|Default|GetMatchDuration))
  ;[1 1 1] Level Start Free For All
  (CallFunction|UpdateGameStateNames)
  (for _array_element (Variables|Default|GetAll_ConnectedControllers)
    (Default|GameStartCountdown _array_element)
    (if (> _matchduration 0)
      (Default|HUDSetupMatchTimer _array_element _matchduration)))
  (Utilities|FlowControl|Delay 3.0)
  (for _array_element_2 (Variables|Default|GetAll_ConnectedControllers)
    (Default|EnableAllInput _array_element_2)
    (Default|HUDStartMatchPVP _array_element_2))
  (if (> (Variables|Default|GetMatchDuration) 0)
    (bind _returnvalue (Utilities|Time|SetTimerbyFunctionName 0 "MatchTimer_Interval" 1.0 true))
    (Variables|Default|SetMatchTimeHandle _returnvalue)))

(event Custom|MatchTimer_Interval
  ;[1 1 1] Match timer interval
  (bind _result (Math|Integer|DecrementInt (Variables|Default|GetMatchDuration))
    (:%20%20
      (Default|UpdateHUDMatchTimer (Variables|Default|GetBP_MPTPS_GameState) _result)
      (if (== (Variables|Default|GetMatchDuration) 0)
        (Development|PrintString "Match Ended")
        (Utilities|Time|ClearandInvalidateTimerbyHandle (Variables|Default|GetMatchTimeHandle))
        (bind _winner (CallFunction|GMPVPFindWinningPlayer))
        (CallFunction|GMPVPGameOver false true _winner)))))

(event Custom|RespawnPoint_Cooldown
  (params (RespawnPoint :type String))
  (Utilities|FlowControl|Delay 3.0)
  (Utilities|Map|Add (Variables|Default|GetAll_RespawnPoints) RespawnPoint false))

(event EventOnLogout
  (params (ExitingController :type Controller%20Object%20Reference))
  ;[1 1 1] LogOut
  (bind _asbp_mptps_player_controller (Utilities|Casting|CastToBP_MPTPS_PlayerController ExitingController))
  (Utilities|Array|RemoveItem (Variables|Default|GetAll_ConnectedControllers) _asbp_mptps_player_controller)
  (Math|Integer|DecrementInt (Variables|Default|GetNum_ExpectedPlayers)
    (:%20%20
      (CallFunction|UpdateGameStateNames))))

(event EventBeginPlay
  ;[0.5935 1 0.4692] BeginPlay
  (CallFunction|SetGameOptions (Variables|Default|GetOptionsString))
  (bind _asbp_mptps_game_state (Utilities|Casting|CastToBP_MPTPS_GameState (Game|GetGameState)))
  (Variables|Default|SetBP_MPTPS_GameState _asbp_mptps_game_state)
  (Variables|Default|SetIsGameModeReady true))

(event EventHandleStartingNewPlayer
  (params (NewPlayer :type Player%20Controller%20Object%20Reference))
  ;[1 1 1] Starting new Player
  (bind _asbp_mptps_player_controller (Utilities|Casting|CastToBP_MPTPS_PlayerController NewPlayer))
  (Default|LoadProfile _asbp_mptps_player_controller)
  (Default|OnControllerSpawned _asbp_mptps_player_controller)
  (Utilities|Array|Add (Variables|Default|GetAll_ConnectedControllers) _asbp_mptps_player_controller)
  (if (Variables|Default|GetIsGameModeReady) :!label _label
    (CallFunction|UpdateGameStateInfo)
    (if (Variables|Default|GetIsSoloGame)
      (bind _allplayersready (CallFunction|CountPlayersSpawned :!label _label_2))
      (if _allplayersready
        (Class|GameModeBase|RestartPlayeratPlayerStart (Utilities|Array|Get(acopy) (Variables|Default|GetAll_ConnectedControllers)) (Class|GameModeBase|FindPlayerStart 0 (Utilities|String|Append (Utilities|String|EnumtoString (Variables|Default|GetGameMode)) "_0")))
        (CallFunction|LevelStartEndlessWave)
        (else
          (Utilities|FlowControl|DelayUntilNextTick)
          (goto _label_2)))
      (elif (== (Variables|Default|GetNum_ExpectedPlayers) (Utilities|Array|Length (Variables|Default|GetAll_ConnectedControllers)))
        (bind _allplayersready_2 (CallFunction|CountPlayersSpawned :!label _label_3))
        (if _allplayersready_2
          (for (_array_element _array_index) (Variables|Default|GetAll_ConnectedControllers)
            (Class|GameModeBase|RestartPlayeratPlayerStart _array_element (Class|GameModeBase|FindPlayerStart _array_element (Utilities|String|Append (Utilities|String|EnumtoString (Variables|Default|GetGameMode)) "_" (Utilities|String|ToString(Integer) _array_index)))))
          (switch Utilities|FlowControl|Switch|SwitchonE_GameModes (Variables|Default|GetGameMode)
            (:NewEnumerator0
              (CallFunction|LevelStartEndlessWave))
            (:NewEnumerator2
              (CallFunction|LevelStartFreeforAll)
              (CallFunction|SetupRespawns)))
          (else
            (Utilities|FlowControl|DelayUntilNextTick)
            (goto _label_3)))))
    (else
      (Utilities|FlowControl|DelayUntilNextTick)
      (goto _label))))

(event EventTick
  (params (DeltaSeconds :type Float%20%28single-precision%29)))

(fn ConstructionScript)

(fn SpawnDefaultPawnfor
  (params (NewPlayer :type Controller%20Object%20Reference) (StartSpot :type Actor%20Object%20Reference))
  (bind _returnvalue (Transformation|GetActorTransform StartSpot))
  (if (Variables|Default|GetSeamlessTravelEnabled)
    (bind _asbp_mptps_player_state (Utilities|Casting|CastToBP_MPTPS_PlayerState (Variables|/Script/Engine.Controller|GetPlayerState NewPlayer)))
    (LocalVariables|SetLocal_PlayerProfileClass (.characterclass (Variables|/Game/Frameworks/BP_MPTPS_PlayerState.BP_MPTPS_PlayerState_C|GetS_PlayerProfile _asbp_mptps_player_state)))
    (LocalVariables|SetLocal_ModelName (.modelname (Variables|/Game/Frameworks/BP_MPTPS_PlayerState.BP_MPTPS_PlayerState_C|GetS_PlayerProfile _asbp_mptps_player_state)))
    (LocalVariables|SetLocal_SkinName (.skinname (Variables|/Game/Frameworks/BP_MPTPS_PlayerState.BP_MPTPS_PlayerState_C|GetS_PlayerProfile _asbp_mptps_player_state)))
    (else
      (bind _asbp_mptps_player_controller (Utilities|Casting|CastToBP_MPTPS_PlayerController NewPlayer))
      (LocalVariables|SetLocal_PlayerProfileClass (.characterclass (Variables|/Game/Frameworks/BP_MPTPS_PlayerController.BP_MPTPS_PlayerController_C|GetS_PlayerProfile _asbp_mptps_player_controller)))
      (LocalVariables|SetLocal_ModelName (.modelname (Variables|/Game/Frameworks/BP_MPTPS_PlayerController.BP_MPTPS_PlayerController_C|GetS_PlayerProfile _asbp_mptps_player_controller)))
      (LocalVariables|SetLocal_SkinName (.skinname (Variables|/Game/Frameworks/BP_MPTPS_PlayerController.BP_MPTPS_PlayerController_C|GetS_PlayerProfile _asbp_mptps_player_controller)))
      (Default|SetSpawnRotation _asbp_mptps_player_controller (.yaw (.Rotation (Math|Transform|BreakTransform _returnvalue))))))
  (bind _returnvalue_2 (Game|SpawnActorfromClass (LocalVariables|GetLocal_PlayerProfileClass) _returnvalue "Undefined" "MultiplyWithRoot" 0 0))
  (bind _asbp_player_base (Utilities|Casting|CastToBP_Player_Base _returnvalue_2))
  (Variables|/Game/Characters/Blueprints/BP_Player_Base.BP_Player_Base_C|SetModelName _asbp_player_base (LocalVariables|GetLocal_ModelName))
  (Variables|/Game/Characters/Blueprints/BP_Player_Base.BP_Player_Base_C|SetSkinName _asbp_player_base (LocalVariables|GetLocal_SkinName))
  (return _asbp_player_base))

(fn RespawnPawnforController
  (params (PlayerController :type BP%20MPTPS%20Player%20Controller%20Object%20Reference) (PlayerStart :type Actor%20Object%20Reference))
  (bind _returnvalue (Transformation|GetActorTransform PlayerStart))
  (bind _s_playerprofile (Variables|/Game/Frameworks/BP_MPTPS_PlayerController.BP_MPTPS_PlayerController_C|GetS_PlayerProfile PlayerController))
  (bind (_characterclass _modelname _skinname) (Utilities|Struct|BreakS_PlayerProfile _s_playerprofile))
  (LocalVariables|SetLocal_PlayerProfileClass _characterclass)
  (LocalVariables|SetLocal_ModelName _modelname)
  (LocalVariables|SetLocal_SkinName _skinname)
  (Default|SetSpawnRotation PlayerController (.yaw (.Rotation (Math|Transform|BreakTransform _returnvalue))))
  (bind _returnvalue_2 (Game|SpawnActorfromClass (LocalVariables|GetLocal_PlayerProfileClass) _returnvalue "Undefined" "MultiplyWithRoot" 0 0))
  (bind _asbp_player_base (Utilities|Casting|CastToBP_Player_Base _returnvalue_2))
  (Variables|/Game/Characters/Blueprints/BP_Player_Base.BP_Player_Base_C|SetModelName _asbp_player_base (LocalVariables|GetLocal_ModelName))
  (Variables|/Game/Characters/Blueprints/BP_Player_Base.BP_Player_Base_C|SetSkinName _asbp_player_base (LocalVariables|GetLocal_SkinName))
  (Variables|/Game/Characters/Blueprints/BP_Player_Base.BP_Player_Base_C|SetDeadRespawn _asbp_player_base true)
  (return _asbp_player_base))

(fn GMEWGetEnemyCount
  (params (WaveNumber :type Integer) (NumberOfPlayers :type Integer))
  (bind _output_get (LocalVariables|SetLocal_NewSpawnCount (+ (+ WaveNumber (* NumberOfPlayers 2)) (Variables|Default|GetGM_EW_EnemiesNumberThisWave))))
  (if (<= _output_get 5)
    (LocalVariables|SetLocal_NewSpawnCount 6))
  (return (LocalVariables|GetLocal_NewSpawnCount)))

(fn GMEWGetEnemyHealth
  (params (WaveNumber :type Integer))
  (if (== WaveNumber 1)
    (LocalVariables|SetLocal_NewHealth 1e+02)
    (else
      (LocalVariables|SetLocal_NewHealth (+ (Variables|Default|GetGM_EW_EnemiesHealthThisWave) 1e+01))))
  (return (LocalVariables|GetLocal_NewHealth)))

(fn GMEWSetupEnemy
  (params (Enemy :type BP%20AI%20Minion%20Base%20Object%20Reference))
  (Variables|/Game/AI/BP_AI_Minion_Base.BP_AI_Minion_Base_C|SetHealth Enemy (Variables|Default|GetGM_EW_EnemiesHealthThisWave))
  (return))

(fn SetGameOptions
  (params (GameOptionString :type String))
  (switch string (Class|GameplayStatics|ParseOption GameOptionString "GameMode")
    (:EndlessWave
      (Variables|Default|SetGameMode "NewEnumerator0"))
    (:FreeForAll
      (Variables|Default|SetGameMode "NewEnumerator2")
      (Variables|Default|SetMatchDuration (Math|Conversions|ToInteger(Byte) (Class|GameplayStatics|ParseOption GameOptionString "MatchDuration")))
      (Variables|Default|SetScoreLimit (Math|Conversions|ToInteger(Byte) (Class|GameplayStatics|ParseOption GameOptionString "ScoreLimit")))
      (Variables|Default|SetRespawnDelay (Math|Conversions|ToInteger(Byte) (Class|GameplayStatics|ParseOption GameOptionString "RespawnDelay")))))
  (Variables|Default|SetNum_ExpectedPlayers (Math|Conversions|ToInteger(Byte) (Class|GameplayStatics|ParseOption GameOptionString "NumConnectedPlayers")))
  (switch string (Class|GameplayStatics|ParseOption GameOptionString "IsSoloGame")
    (:True
      (Variables|Default|SetIsSoloGame true))
    (:False
      (Variables|Default|SetIsSoloGame false)))
  (switch string (Class|GameplayStatics|ParseOption GameOptionString "UseSeamlessTravel")
    (:True
      ;[1 1 1] Custom boolean
      (Variables|Default|SetSeamlessTravelEnabled true)
      ;[1 1 1] Class default
      (Variables|Default|SetbUseSeamlessTravel true))
    (:False
      (Variables|Default|SetSeamlessTravelEnabled false)
      (Variables|Default|SetbUseSeamlessTravel false)))
  (return))

(fn GMEWPlayerDied
  (for _array_element (Variables|Default|GetAll_ConnectedControllers)
    (bind _asbp_player_base (Utilities|Casting|CastToBP_Player_Base (Pawn|GetControlledPawn _array_element))
      (:then
        (if (not (Variables|/Game/Characters/Blueprints/BP_Player_Base.BP_Player_Base_C|GetIsAlive _asbp_player_base))
          (Math|Integer|IncrementInt (LocalVariables|GetLocal_DeadPlayerCount) :!label _label)))
      (:CastFailed
        (if (Variables|/Game/Frameworks/BP_MPTPS_PlayerController.BP_MPTPS_PlayerController_C|GetIsSpectating _array_element)
          (goto _label)))))
  (if (== (LocalVariables|GetLocal_DeadPlayerCount) (Utilities|Array|Length (Variables|Default|GetAll_ConnectedControllers)))
    (CallFunction|GMEWGameOver))
  (return))

(fn CountPlayersSpawned
  (for _array_element (Variables|Default|GetAll_ConnectedControllers)
    (if (Variables|/Game/Frameworks/BP_MPTPS_PlayerController.BP_MPTPS_PlayerController_C|GetIsPlayerSpawned _array_element)
      (Math|Integer|IncrementInt (LocalVariables|GetLocal_PlayersReady))))
  (return (== (Utilities|Array|Length (Variables|Default|GetAll_ConnectedControllers)) (LocalVariables|GetLocal_PlayersReady))))

(fn UpdateGameStateNames
  (for (_array_element _array_index) (Variables|Default|GetAll_ConnectedControllers)
    (Utilities|Array|SetArrayElem (LocalVariables|GetLocal_AllPlayerNames) _array_index (Utilities|Struct|BreakS_PlayerProfile (Variables|/Game/Frameworks/BP_MPTPS_PlayerController.BP_MPTPS_PlayerController_C|GetS_PlayerProfile _array_element)) true))
  (Default|UpdateHUDPlayerNames (Variables|Default|GetBP_MPTPS_GameState) (LocalVariables|GetLocal_AllPlayerNames)))

(fn SetupRespawns
  (LocalVariables|SetLocal_GameModeString (Utilities|String|EnumtoString (Variables|Default|GetGameMode)))
  (bind _outactors (Actor|GetAllActorsOfClass "/Script/Engine.PlayerStart"))
  (for _array_element _outactors
    (if (>= (Utilities|String|FindSubstring (Utilities|String|ToString(Name) (Variables|/Script/Engine.PlayerStart|GetPlayerStartTag _array_element)) (LocalVariables|GetLocal_GameModeString)) 0)
      (Utilities|Map|Add (Variables|Default|GetAll_RespawnPoints) (Utilities|String|ToString(Name) (Variables|/Script/Engine.PlayerStart|GetPlayerStartTag _array_element)) false))))

(fn RespawnAfterDying
  (params (PlayerController :type BP%20MPTPS%20Player%20Controller%20Object%20Reference%20%28by%20ref%29))
  (bind _keys (Utilities|Map|Keys (Variables|Default|GetAll_RespawnPoints)))
  (bind _output_get (LocalVariables|SetLocal_All_RespawnPoints _keys))
  (LocalVariables|SetLocal_PickedRespawnPoint (.OutItem (Utilities|Array|Random _output_get)) :!label _label)
  (bind _result (Math|Integer|IncrementInt (LocalVariables|GetLocal_LoopCount))
    (:%20%20
      (if (<= _result 10)
        (if (.Value (Utilities|Map|Find (Variables|Default|GetAll_RespawnPoints) (LocalVariables|GetLocal_PickedRespawnPoint)))
          (goto _label)
          (else
            _)))
      (Utilities|Map|Add (Variables|Default|GetAll_RespawnPoints) (LocalVariables|GetLocal_PickedRespawnPoint) true)
      (CallFunction|RespawnPointCooldown (LocalVariables|GetLocal_PickedRespawnPoint))
      (Pawn|UnPossess PlayerController)
      (bind _playerbase (CallFunction|RespawnPawnforController PlayerController (Class|GameModeBase|FindPlayerStart PlayerController (LocalVariables|GetLocal_PickedRespawnPoint))))
      (Pawn|Possess PlayerController _playerbase))))

(fn GMPVPKillPlayer
  (params (Killer :type BP%20MPTPS%20Player%20Controller%20Object%20Reference) (Victim :type BP%20MPTPS%20Player%20Controller%20Object%20Reference))
  (bind _result (Math|Integer|IncrementInt (Variables|/Game/Frameworks/BP_MPTPS_PlayerController.BP_MPTPS_PlayerController_C|GetKills Killer))
    (:%20%20
      (Variables|/Game/Frameworks/BP_MPTPS_PlayerState.BP_MPTPS_PlayerState_C|SetKills (Variables|/Game/Frameworks/BP_MPTPS_PlayerController.BP_MPTPS_PlayerController_C|GetBP_MPTPS_PlayerState Killer) _result)
      (bind _result_2 (Math|Integer|IncrementInt (Variables|/Game/Frameworks/BP_MPTPS_PlayerController.BP_MPTPS_PlayerController_C|GetDeaths Victim))
        (:%20%20
          (bind _output_get (Variables|/Game/Frameworks/BP_MPTPS_PlayerState.BP_MPTPS_PlayerState_C|SetDeaths (Variables|/Game/Frameworks/BP_MPTPS_PlayerController.BP_MPTPS_PlayerController_C|GetBP_MPTPS_PlayerState Victim) _result_2))
          (if (and (== _output_get (Variables|Default|GetScoreLimit)) (> (Variables|Default|GetScoreLimit) 0))
            (CallFunction|GMPVPGameOver true false Killer)
            (else
              (LocalVariables|SetLocal_VictimName (.PlayerName (Utilities|Struct|BreakS_PlayerProfile (Variables|/Game/Frameworks/BP_MPTPS_PlayerController.BP_MPTPS_PlayerController_C|GetS_PlayerProfile Victim))))
              (LocalVariables|SetLocal_KillerName (.PlayerName (Utilities|Struct|BreakS_PlayerProfile (Variables|/Game/Frameworks/BP_MPTPS_PlayerController.BP_MPTPS_PlayerController_C|GetS_PlayerProfile Killer))))
              (Default|UIShowKillMessage Killer true (LocalVariables|GetLocal_VictimName))
              (Default|UIShowKillMessage Victim false "" (LocalVariables|GetLocal_KillerName))
              (LocalVariables|SetLocal_NewsFeedLine (Utilities|Text|FormatText "{a} killed {b}" (LocalVariables|GetLocal_KillerName) (LocalVariables|GetLocal_VictimName)))
              (for _array_element (Variables|Default|GetAll_ConnectedControllers)
                (Default|UIUpdateNewsFeed _array_element (LocalVariables|GetLocal_NewsFeedLine))))))))))

(fn UpdateGameStateInfo
  (bind _bp_mptps_gamestate (Variables|Default|GetBP_MPTPS_GameState))
  (Variables|/Game/Frameworks/BP_MPTPS_GameState.BP_MPTPS_GameState_C|SetCurrentGameMode _bp_mptps_gamestate (Variables|Default|GetGameMode))
  (Variables|/Game/Frameworks/BP_MPTPS_GameState.BP_MPTPS_GameState_C|SetScoreLimit _bp_mptps_gamestate (Variables|Default|GetScoreLimit))
  (Variables|/Game/Frameworks/BP_MPTPS_GameState.BP_MPTPS_GameState_C|SetMatchDuration _bp_mptps_gamestate (Variables|Default|GetMatchDuration)))

(fn GMPVPFindWinningPlayer
  (for (_array_element _array_index) (Variables|Default|GetAll_ConnectedControllers)
    (Utilities|Array|SetArrayElem (LocalVariables|GetLocal_KillScores) _array_index (Variables|/Game/Frameworks/BP_MPTPS_PlayerController.BP_MPTPS_PlayerController_C|GetKills _array_element) true))
  (return (Utilities|Array|Get(acopy) (Variables|Default|GetAll_ConnectedControllers) (.IndexOfMaxValue (Math|Integer|MaxOfIntArray (LocalVariables|GetLocal_KillScores))))))