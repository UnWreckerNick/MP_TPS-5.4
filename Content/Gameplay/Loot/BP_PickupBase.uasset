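; Base actor for loot pickups, configured per row from the DR_PickupInfo data table.
; The construction script sets the name, static or fallback skeletal mesh with scale and offset, name widget offset, and hint and auto-pickup flags.
; At BeginPlay it writes the name into the WB_PickupItemName widget, whose visibility can be toggled when names are enabled.
; Getters expose auto-pickup and the interaction hint, which is suppressed for auto-pickups.
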(event EventBeginPlay
  (bind _aswb_pickup_item_name (Utilities|Casting|CastToWB_PickupItemName (UserInterface|GetUserWidgetObject (Variables|Default|GetWidget_PickupName))))
  (Default|SetTextPickupMenu _aswb_pickup_item_name (Variables|Default|GetPickupName)))

(event EventSetItemNameVisibility
  (params (NewVisibility :type Boolean))
  (if (Variables|Default|GetShowPickupName)
    (Rendering|SetVisibility (Variables|Default|GetWidget_PickupName) NewVisibility false)))

(fn ConstructionScript
  (bind _pickupmesh (Variables|Default|GetPickupMesh))
  (bind _pickupmesh_skeletal (Variables|Default|GetPickupMesh_Skeletal))
  (bind _returnvalue (Utilities|GetDataTableRow "/Game/Gameplay/Loot/DR_PickupInfo.DR_PickupInfo" (Variables|Default|GetPickupRowName))
    (:then
      (Variables|Default|SetPickupName (.PickupName (Utilities|Struct|BreakS_PickupInfo _returnvalue)))
      (if (!= (.PickupMesh (Utilities|Struct|BreakS_PickupInfo _returnvalue)) 0)
        (Components|StaticMesh|SetStaticMesh _pickupmesh (.PickupMesh (Utilities|Struct|BreakS_PickupInfo _returnvalue)))
        (Transformation|SetRelativeScale3D _pickupmesh (Math|Vector|MakeVector (.PickupMesh_Scale (Utilities|Struct|BreakS_PickupInfo _returnvalue)) (.PickupMesh_Scale (Utilities|Struct|BreakS_PickupInfo _returnvalue)) (.PickupMesh_Scale (Utilities|Struct|BreakS_PickupInfo _returnvalue))))
        (Transformation|SetRelativeLocation _pickupmesh (.PickupMesh_Offset (Utilities|Struct|BreakS_PickupInfo _returnvalue)) false false)
        (else
          (Components|SkeletalMesh|SetSkeletalMeshAsset _pickupmesh_skeletal (.PickMesh_Skeletal (Utilities|Struct|BreakS_PickupInfo _returnvalue)))
          (Transformation|SetRelativeScale3D _pickupmesh_skeletal (Math|Vector|MakeVector (.PickupMesh_Scale (Utilities|Struct|BreakS_PickupInfo _returnvalue)) (.PickupMesh_Scale (Utilities|Struct|BreakS_PickupInfo _returnvalue)) (.PickupMesh_Scale (Utilities|Struct|BreakS_PickupInfo _returnvalue))))
          (Transformation|SetRelativeLocation _pickupmesh_skeletal (.PickupMesh_Offset (Utilities|Struct|BreakS_PickupInfo _returnvalue)) false false)))
      (Transformation|AddLocalOffset (Variables|Default|GetWidget_PickupName) (.PickupMesh_Offset (Utilities|Struct|BreakS_PickupInfo _returnvalue)) false false)
      (Variables|Default|SetShowPickupName (.ShowPickupName (Utilities|Struct|BreakS_PickupInfo _returnvalue)))
      (Variables|Default|SetInteractableHint (.InteractableHint (Utilities|Struct|BreakS_PickupInfo _returnvalue)))
      (Variables|Default|SetShowInteractableHint (.ShowInteractableHint (Utilities|Struct|BreakS_PickupInfo _returnvalue)))
      (Variables|Default|SetAutoPickUp (.IsAutoPickup (Utilities|Struct|BreakS_PickupInfo _returnvalue))))))

(fn GetInteractionHint
  (if (Variables|Default|GetAutoPickUp)
    (LocalVariables|SetLocal_ShowHint false :!label _label)
    (elif (Variables|Default|GetShowInteractableHint)
      (LocalVariables|SetLocal_ShowHint true)
      (else
        (goto _label))))
  (return (Variables|Default|GetInteractableHint) (LocalVariables|GetLocal_ShowHint)))

(fn IsAutoPickup
  (return (Variables|Default|GetAutoPickUp)))