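; Weapon and ammo pickup that destroys itself when a player successfully collects it.
; Construction reads DT_PickupInfo to strip either the meshes or the particle system by pickup type.
; Pickup adds unowned weapons using DT_WeaponInfo limits and switches to them, but rejects ammo for unowned weapons.
; It fills ammo (-1 means max), spills clip overflow into stock, and uses RPCs for inventory, active-weapon HUD and optional saving.
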(event EventInteractwithActor
  (params (PlayerCharacter :type BP%20Player%20Base%20Object%20Reference))
  (bind _isitempickedup (CallFunction|Pickup PlayerCharacter))
  (if _isitempickedup
    (Actor|DestroyActor)))

(fn ConstructionScript
  (|CallParentFunction)
  (bind _returnvalue (Utilities|GetDataTableRow "/Game/Gameplay/Loot/DT_PickupInfo.DT_PickupInfo" (Variables|Default|GetPickupRowName))
    (:then
      (if (.IsAmmoPickUp (Utilities|Struct|BreakS_PickupInfo _returnvalue))
        (Components|DestroyComponent (Variables|Default|GetPickupMesh_Skeletal))
        (else
          (Components|DestroyComponent (Variables|Default|GetParticleSystem)))))))

(fn Pickup
  (params (Player :type BP%20Player%20Base%20Object%20Reference))
  (bind (_slottoaddweapon _isownedweapon) (Default|FindWeaponSlot Player (Variables|Default|GetWeaponRowNameToAdd)))
  (LocalVariables|SetLocal_WeaponInventorySlot _slottoaddweapon)
  (LocalVariables|SetLocal_IsNewWeapon (not _isownedweapon))
  (if (and (LocalVariables|GetLocal_IsNewWeapon) (Variables|Default|GetIsAmmoPickup))
    (LocalVariables|SetLocal_IsItemPickedup false)
    (else
      (LocalVariables|SetLocal_IsItemPickedup true)
      (bind _returnvalue (Utilities|GetDataTableRow "/Game/Weapons/DT_WeaponInfo.DT_WeaponInfo" (Variables|Default|GetWeaponRowNameToAdd))
        (:then
          (if (and (LocalVariables|GetLocal_IsNewWeapon) (not (Variables|Default|GetIsAmmoPickup)))
            (Default|ServerAddWeapontoInventory Player (LocalVariables|GetLocal_WeaponInventorySlot) (Variables|Default|GetWeaponRowNameToAdd)))
          (if (LocalVariables|GetLocal_IsNewWeapon)
            (LocalVariables|SetLocal_CurrentClip 0)
            (LocalVariables|SetLocal_CurrentClipMaximum (.AmmoClip (Utilities|Struct|BreakS_WeaponInfo _returnvalue)))
            (LocalVariables|SetLocal_CurrentStock 0)
            (LocalVariables|SetLocal_CurrentStockMaximum (.AmmoStock (Utilities|Struct|BreakS_WeaponInfo _returnvalue)))
            (else
              (LocalVariables|SetLocal_CurrentClip (Utilities|Array|Get(acopy) (Variables|/Game/Characters/Blueprints/BP_Player_Base.BP_Player_Base_C|GetAmmoClip Player) (LocalVariables|GetLocal_WeaponInventorySlot)))
              (LocalVariables|SetLocal_CurrentClipMaximum (Utilities|Array|Get(acopy) (Variables|/Game/Characters/Blueprints/BP_Player_Base.BP_Player_Base_C|GetAmmoClipMax Player) (LocalVariables|GetLocal_WeaponInventorySlot)))
              (LocalVariables|SetLocal_CurrentStock (Utilities|Array|Get(acopy) (Variables|/Game/Characters/Blueprints/BP_Player_Base.BP_Player_Base_C|GetAmmoStock Player) (LocalVariables|GetLocal_WeaponInventorySlot)))
              (LocalVariables|SetLocal_CurrentStockMaximum (Utilities|Array|Get(acopy) (Variables|/Game/Characters/Blueprints/BP_Player_Base.BP_Player_Base_C|GetAmmoStockMax Player) (LocalVariables|GetLocal_WeaponInventorySlot)))))
          (if (== (Variables|Default|GetLoaded_Ammo_Clip) -1)
            (Utilities|Array|SetArrayElem (Variables|/Game/Characters/Blueprints/BP_Player_Base.BP_Player_Base_C|GetAmmoClip Player) (LocalVariables|GetLocal_WeaponInventorySlot) (LocalVariables|GetLocal_CurrentClipMaximum))
            (else
              (LocalVariables|SetLocal_ClipOverflow (Math|Integer|Clamp(Integer) (- (+ (Variables|Default|GetLoaded_Ammo_Clip) (LocalVariables|GetLocal_CurrentClip)) (LocalVariables|GetLocal_CurrentClipMaximum)) 0 999999))
              (Utilities|Array|SetArrayElem (Variables|/Game/Characters/Blueprints/BP_Player_Base.BP_Player_Base_C|GetAmmoClip Player) (LocalVariables|GetLocal_WeaponInventorySlot) (Math|Integer|Clamp(Integer) (+ (Variables|Default|GetLoaded_Ammo_Clip) (LocalVariables|GetLocal_CurrentClip)) 0 (LocalVariables|GetLocal_CurrentClipMaximum)))))
          (if (== (Variables|Default|GetLoaded_Ammo_Stock) -1)
            (Utilities|Array|SetArrayElem (Variables|/Game/Characters/Blueprints/BP_Player_Base.BP_Player_Base_C|GetAmmoStock Player) (LocalVariables|GetLocal_WeaponInventorySlot) (LocalVariables|GetLocal_CurrentStockMaximum))
            (else
              (Utilities|Array|SetArrayElem (Variables|/Game/Characters/Blueprints/BP_Player_Base.BP_Player_Base_C|GetAmmoStock Player) (LocalVariables|GetLocal_WeaponInventorySlot) (Math|Integer|Clamp(Integer) (+ (Variables|Default|GetLoaded_Ammo_Stock) (LocalVariables|GetLocal_CurrentStock) (LocalVariables|GetLocal_ClipOverflow)) 0 (LocalVariables|GetLocal_CurrentStockMaximum)))))
          (if (and (or (Variables|Default|GetIsAmmoPickup) (and (not (LocalVariables|GetLocal_IsNewWeapon)) (not (Variables|Default|GetIsAmmoPickup)))) (== (LocalVariables|GetLocal_WeaponInventorySlot) (Variables|/Game/Characters/Blueprints/BP_Player_Base.BP_Player_Base_C|GetActiveWeaponIndex Player)))
            (Default|ClientUpdateHUDClip Player (Utilities|Array|Get(acopy) (Variables|/Game/Characters/Blueprints/BP_Player_Base.BP_Player_Base_C|GetAmmoClip Player) (LocalVariables|GetLocal_WeaponInventorySlot)))
            (Default|ClientUpdateHUDStock Player (Utilities|Array|Get(acopy) (Variables|/Game/Characters/Blueprints/BP_Player_Base.BP_Player_Base_C|GetAmmoStock Player) (LocalVariables|GetLocal_WeaponInventorySlot))))
          (if (and (Variables|Default|GetSavedPickedupWeapon) (not (Variables|Default|GetIsAmmoPickup)))
            (Default|ClientSavePickedupWeapon (Variables|/Game/Characters/Blueprints/BP_Player_Base.BP_Player_Base_C|GetBP_MPTPS%20PlayerController Player) (Variables|Default|GetWeaponRowNameToAdd)))
          (if (and (LocalVariables|GetLocal_IsNewWeapon) (not (Variables|Default|GetIsAmmoPickup)))
            (Default|MulticastSwitchWeapon Player (LocalVariables|GetLocal_WeaponInventorySlot)))))))
  (return (LocalVariables|GetLocal_IsItemPickedup)))