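; Base AI controller for minions that makes them chase players they see.
; On possess it caches the pawn as BP_AI_Minion_Base, and perception updates are filtered to the sight sense.
; A sighted player becomes the minion's target and move goal only while switching is allowed.
; Switching locks on acquisition or while TargetPlayer is seen, and unlocks when sight of TargetPlayer is lost.
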(event OnTargetPerceptionUpdated(AIPerception)
  (params (Actor :type Actor%20Object%20Reference) (Stimulus :type AI%20Stimulus%20Structure))
  (bind _bsuccessfullysensed (Utilities|Struct|BreakAIStimulus Stimulus))
  (bind _bp_ai_minion_base (Variables|Default|GetBP%20AI%20Minion%20Base))
  (bind _returnvalue (Class|AIPerceptionSystem|GetSenseClassforStimulus Stimulus))
  (if (== _returnvalue "/Script/AIModule.AISense_Sight")
    (if (!= Actor (Variables|Default|GetTargetPlayer))
      (bind _asbp_player_base (Utilities|Casting|CastToBP_Player_Base Actor))
      (if _bsuccessfullysensed
        (if (Variables|Default|GetCanSwitchTarget)
          (Variables|Default|SetCanSwitchTarget false)
          (Default|SetTargetPlayer _bp_ai_minion_base _asbp_player_base)
          (Default|MovetoPlayer _bp_ai_minion_base)))
      (elif _bsuccessfullysensed
        (Variables|Default|SetCanSwitchTarget false)
        (else
          (Variables|Default|SetCanSwitchTarget true))))))

(event EventBeginPlay)

(event EventTick
  (params (DeltaSeconds :type Float%20%28single-precision%29)))

(event EventPossess
  (params (PossessedPawn :type Pawn%20Object%20Reference))
  (bind _asbp_ai_minion_base (Utilities|Casting|CastToBP_AI_Minion_Base PossessedPawn))
  (Variables|Default|SetBP%20AI%20Minion%20Base _asbp_ai_minion_base))

(fn ConstructionScript)