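; Player component that tracks XP and level in a multiplayer game, starting from values in the player controller's profile.
; Multicast XP gains apply only on the server and owning client, checking a level threshold map to allow capped, possibly multi-level jumps.
; Results are written back to the profile of player controller 0, while the local player also refreshes the HUD, saves progress and plays a level-up animation.
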(event Custom|XPComponentInit
  (CallFunction|SetXPMap)
  (bind _asbp_player_base (Utilities|Casting|CastToBP_Player_Base (Components|GetOwner)))
  (Variables|Default|SetBP%20Player%20Base _asbp_player_base)
  (bind _asbp_mptps_player_controller (Utilities|Casting|CastToBP_MPTPS_PlayerController (Game|GetPlayerController 0)))
  (bind _output_get (Variables|Default|SetBP%20MPTPS%20Player%20Controller _asbp_mptps_player_controller))
  (Variables|Default|SetPlayer%20XP (.playerxp (Variables|/Game/Frameworks/BP_MPTPS_PlayerController.BP_MPTPS_PlayerController_C|GetS_PlayerProfile _output_get)))
  (Variables|Default|SetPlayer%20Level (.playerlevel (Variables|/Game/Frameworks/BP_MPTPS_PlayerController.BP_MPTPS_PlayerController_C|GetS_PlayerProfile _output_get)))
  (if (Pawn|IsLocalPlayerController (Variables|Default|GetBP%20MPTPS%20Player%20Controller))
    (Default|UpdateXPAmount (Variables|/Game/Frameworks/BP_MPTPS_PlayerController.BP_MPTPS_PlayerController_C|GetWB_IngameHUD (Variables|Default|GetBP%20MPTPS%20Player%20Controller)))
    (Default|UpdateXPLevel (Variables|/Game/Frameworks/BP_MPTPS_PlayerController.BP_MPTPS_PlayerController_C|GetWB_IngameHUD (Variables|Default|GetBP%20MPTPS%20Player%20Controller)))
    (Default|SaveXPandLevel (Variables|Default|GetBP%20MPTPS%20Player%20Controller))))

(event Custom|Multicast_ComponentAddXP
  (params (XPAmount :type Integer))
  (bind _bp_player_base (Variables|Default|GetBP%20Player%20Base))
  (bind _wb_ingame_hud (Variables|/Game/Characters/Blueprints/BP_Player_Base.BP_Player_Base_C|GetWB%20Ingame%20HUD _bp_player_base))
  (if (or (Networking|IsServer) (Pawn|IsLocallyControlled (Variables|Default|GetBP%20Player%20Base)))
    (bind _output_get (Variables|Default|SetPlayer%20XP (+ XPAmount (Variables|Default|GetPlayer%20XP))))
    (bind (_canlevelup _newlevel) (CallFunction|CheckforLevelUp _output_get))
    (if _canlevelup
      (Variables|Default|SetPlayer%20Level _newlevel))
    (CallFunction|UpdatePlayerControllerProfile)
    (if (Pawn|IsLocallyControlled _bp_player_base)
      (Default|UpdateXPAmount _wb_ingame_hud)
      (Default|UpdateXPLevel _wb_ingame_hud)
      (Default|SaveXPandLevel (Variables|Default|GetBP%20MPTPS%20Player%20Controller))
      (if _canlevelup
        (Default|PlayUILevelUpAnim (Variables|/Game/Frameworks/BP_MPTPS_PlayerController.BP_MPTPS_PlayerController_C|GetWB_IngameHUD (Variables|Default|GetBP%20MPTPS%20Player%20Controller)))))))

(fn SetXPMap
  (Variables|Default|SetXP%20Map%20Levels (.xp_map_levels (LocalVariables|GetS_XPAndLevel)))
  (return))

(fn CheckforLevelUp
  (params (XPAmount :type Integer))
  (LocalVariables|SetLocal_CurrentPlayerXP XPAmount)
  (LocalVariables|SetLocal_CurrentPlayerLevel (Variables|Default|GetPlayer%20Level))
  (if (and (> (Variables|Default|GetPlayer%20XP) (Utilities|Array|Get(acopy) (Variables|Default|GetXP%20Map%20Levels) (LocalVariables|GetLocal_CurrentPlayerLevel))) (< (LocalVariables|GetLocal_CurrentPlayerLevel) 10))
    (LocalVariables|SetLocal_CanLevelUp true)
    (bind _index (Utilities|FlowControl|ForLoopwithBreak (LocalVariables|GetLocal_CurrentPlayerLevel) 11 :!label _label)
      (:LoopBody
        (if (not (> (LocalVariables|GetLocal_CurrentPlayerXP) (Utilities|Array|Get(acopy) (Variables|Default|GetXP%20Map%20Levels) _index)))
          (LocalVariables|SetLocal_CurrentPlayerLevel _index)
          (goto _label Break)))
      (:Completed
        (return (LocalVariables|GetLocal_CanLevelUp) (LocalVariables|GetLocal_CurrentPlayerLevel))))
    (else
      (LocalVariables|SetLocal_CanLevelUp false)
      (return (LocalVariables|GetLocal_CanLevelUp) (LocalVariables|GetLocal_CurrentPlayerLevel)))))

(fn UpdatePlayerControllerProfile
  (Utilities|Struct|SetmembersinS_PlayerProfile (Variables|/Game/Frameworks/BP_MPTPS_PlayerController.BP_MPTPS_PlayerController_C|GetS_PlayerProfile (Variables|Default|GetBP%20MPTPS%20Player%20Controller)) (Variables|Default|GetPlayer%20XP) (Variables|Default|GetPlayer%20Level))
  (return))